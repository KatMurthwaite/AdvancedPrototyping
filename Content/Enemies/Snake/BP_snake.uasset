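; Snake enemy that tells its AI behavior through the blackboard whether it can see the player.
; PawnSensing sightings of the third-person character set CanSeePlayer, and a retriggerable delay clears it shortly after sightings stop.
; LaunchSnake sets the capsule location with a single VInterpTo from the given target toward the capsule, whose clamped step resolves to the capsule's current location, leaving it in place.
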(event OnSeePawn(PawnSensing)
  (params (Pawn :type Pawn%20Object%20Reference))
  (Utilities|Casting|CastToBP_ThirdPersonCharacter Pawn)
  (AI|Components|Blackboard|SetValueasBool (AI|GetBlackboard (AI|GetAIController self)) (Utilities|Name|MakeLiteralName "CanSeePlayer") true)
  (Utilities|FlowControl|RetriggerableDelay 0.6)
  (Utilities|Casting|CastToBP_ThirdPersonCharacter Pawn)
  (AI|Components|Blackboard|SetValueasBool (AI|GetBlackboard (AI|GetAIController self)) (Utilities|Name|MakeLiteralName "CanSeePlayer") false))

(event EventBeginPlay)

(event Collision|EventActorBeginOverlap
  (params (OtherActor :type Actor%20Object%20Reference)))

(event EventTick
  (params (DeltaSeconds :type Float%20%28single-precision%29)))

(fn ConstructionScript)

(fn LaunchSnake
  (params (target :type Vector))
  (bind _capsulecomponent (Variables|Collision|GetCapsuleComponent))
  (Transformation|SetWorldLocation _capsulecomponent (Math|Interpolation|VInterpTo target (Transformation|GetWorldLocation _capsulecomponent) 0.16 7e+02) false false))