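; Rooster enemy that chases and pecks the player, and is destroyed when its health runs out.
; PawnSensing sightings call Attack and set a spotted flag, which a retriggerable delay clears once sightings stop.
; While spotted, Tick speeds it up, chases via AIMoveTo and starts cooldown-gated attacks.
; Attack tints the mesh red and deals rate-limited, in-range pecks, restoring white and ending after a set count.
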(event OnSeePawn(PawnSensing)
  (params (Pawn :type Pawn%20Object%20Reference))
  (Variables|Default|SetplayerSpotted true)
  (CallFunction|Attack)
  (Utilities|FlowControl|RetriggerableDelay 0.6)
  (Variables|Default|SetplayerSpotted false))

(event Custom|RunAtPlayer
  (AI|AIMoveTo self "0, 0, 0" (Game|GetPlayerCharacter 0) 5.0 true))

(event Custom|TakeDamage
  (params (Damage :type Float%20%28double-precision%29))
  (bind _output_get (Variables|Default|SetHealth (- (Variables|Default|GetHealth) Damage)))
  (if (<= _output_get 0.0)
    (Actor|DestroyActor)))

(event Custom|Attack
  (bind _returnvalue (Game|GetPlayerCharacter 0))
  ;[1 1 1] Attack System
  (bind _returnvalue_2 (Rendering|Material|CreateDynamicMaterialInstance (Variables|Character|GetMesh) 0 0 "None" :!class /Script/Engine.PrimitiveComponent))
  (Rendering|Material|SetVectorParameterValue _returnvalue_2 "RoosterColour" (Utilities|Struct|MakeLinearColor 1.0 0.0 0.0 0.0) :!class /Script/Engine.MaterialInstanceDynamic)
  (if (and (< (Transformation|GetDistanceTo _returnvalue) (Variables|Default|GetAttackRange)) (> (Utilities|Time|GetTimeSeconds) (+ (Variables|Default|GetlastPeck) (Variables|Default|GetpeckCooldown))))
    (CallFunction|DoDamage _returnvalue)
    (Math|Integer|IncrementInt (Variables|Default|GetpeckCount)
      (:%20%20
        (if (>= (Variables|Default|GetpeckCount) (Variables|Default|GetpecksPerAtt))
          (Variables|Default|SetpeckCount 0)
          (Variables|Default|Setattacking false)
          (bind _returnvalue_3 (Rendering|Material|CreateDynamicMaterialInstance (Variables|Character|GetMesh) 0 0 "None" :!class /Script/Engine.PrimitiveComponent))
          (Rendering|Material|SetVectorParameterValue _returnvalue_3 "RoosterColour" (Utilities|Struct|MakeLinearColor 1.0 1.0 1.0 0.0) :!class /Script/Engine.MaterialInstanceDynamic))))))

(event Custom|DoDamage
  (params (Target :type Pawn%20Object%20Reference))
  ;[1 1 1] Attack System
  (bind _asbp_third_person_character (Utilities|Casting|CastToBP_ThirdPersonCharacter Target))
  (Default|TakeDamage _asbp_third_person_character (Variables|Default|Getdamage)))

(event EventBeginPlay
  (Variables|/Script/Engine.CharacterMovementComponent|SetMaxWalkSpeed (Variables|Character|GetCharacterMovement) (Variables|Default|GetpassiveSpeed)))

(event Collision|EventActorBeginOverlap
  (params (OtherActor :type Actor%20Object%20Reference)))

(event EventTick
  (params (DeltaSeconds :type Float%20%28single-precision%29))
  (Utilities|FlowControl|Sequence
    (:then_0
      (if (Variables|Default|GetplayerSpotted)
        (Variables|/Script/Engine.CharacterMovementComponent|SetMaxWalkSpeed (Variables|Character|GetCharacterMovement) (Variables|Default|GetactiveSpeed))
        (CallFunction|RunatPlayer)
        (if (> (Utilities|Time|GetTimeSeconds) (+ (Variables|Default|GetlastAttack) (Variables|Default|GetattackCooldown)))
          (Variables|Default|SetlastAttack (Utilities|Time|GetTimeSeconds))
          (Variables|Default|Setattacking true))
        (else
          (Variables|/Script/Engine.CharacterMovementComponent|SetMaxWalkSpeed (Variables|Character|GetCharacterMovement) (Variables|Default|GetpassiveSpeed)))))
    (:then_1
      (if (Variables|Default|Getattacking)
        (CallFunction|Attack)))))

(fn ConstructionScript)