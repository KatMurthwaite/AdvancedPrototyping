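; Rooster turret enemy that spins at a random rate while searching and reacts when PawnSensing spots a pawn, resuming search after a short retriggerable delay.
; While spotted, Tick turns it toward the player, pitching ProjectileSpawn and flipping the mesh to face away out of range or toward in range, where it fires cooldown-limited projectiles.
; Only player-caused damage reduces health, destroying it at zero.
; FlashColour briefly tints a dynamic material.
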(event OnSeePawn(PawnSensing)
  (params (Pawn :type Pawn%20Object%20Reference))
  (Variables|Default|SetSpotted%20Player true)
  (Variables|Default|SetSearching false)
  (Utilities|FlowControl|RetriggerableDelay 0.6)
  (Variables|Default|SetSpotted%20Player false)
  (Variables|Default|SetSearching true))

(event Custom|FacePlayer
  (bind _returnvalue (Transformation|GetActorLocation))
  (bind _returnvalue_2 (Game|GetPlayerCharacter 0))
  (bind _returnvalue_3 (Transformation|GetActorLocation _returnvalue_2))
  (bind _returnvalue_4 (Math|Rotator|FindLookatRotation _returnvalue _returnvalue_3))
  (Transformation|SetActorRotation (Math|Rotator|MakeRotator (.roll _returnvalue_4) 0.0 (.yaw _returnvalue_4)))
  (Transformation|SetRelativeRotation (Variables|Default|GetProjectileSpawn) (Math|Rotator|MakeRotator 0.0 (.pitch _returnvalue_4) 0.0) false false)
  (Transformation|SetRelativeRotation (Variables|Character|GetMesh) (Math|Rotator|MakeRotator 0.0 0.0 -9e+01) false false))

(event Custom|TakeDamage
  (params (Damage :type Float%20%28double-precision%29))
  (bind _output_get (Variables|Default|SetHealth (- (Variables|Default|GetHealth) Damage)))
  (if (<= _output_get 0.0)
    (Actor|DestroyActor)))

(event Custom|AimAtPlayer
  (bind _returnvalue (Transformation|GetActorLocation))
  (bind _returnvalue_2 (Game|GetPlayerCharacter 0))
  (bind _returnvalue_3 (Transformation|GetActorLocation _returnvalue_2))
  (bind _returnvalue_4 (Math|Rotator|FindLookatRotation _returnvalue _returnvalue_3))
  (Transformation|SetActorRotation (Math|Rotator|MakeRotator (.roll _returnvalue_4) 0.0 (.yaw _returnvalue_4)))
  (Transformation|SetRelativeRotation (Variables|Default|GetProjectileSpawn) (Math|Rotator|MakeRotator 0.0 (.pitch _returnvalue_4) 0.0) false false)
  (Transformation|SetRelativeRotation (Variables|Character|GetMesh) (Math|Rotator|MakeRotator 0.0 0.0 9e+01) false false))

(event Custom|FlashColour
  (params (Colour :type Linear%20Color%20Structure))
  (bind _returnvalue (Rendering|Material|CreateDynamicMaterialInstance (Variables|Character|GetMesh) 0 0 "None" :!class /Script/Engine.PrimitiveComponent))
  (Rendering|Material|SetVectorParameterValue _returnvalue "RoosterFlashColour" Colour :!class /Script/Engine.MaterialInstanceDynamic)
  (Utilities|FlowControl|RetriggerableDelay 0.1)
  (Rendering|Material|SetVectorParameterValue _returnvalue "RoosterFlashColour" "(R=0.000000,G=0.000000,B=0.000000,A=1.000000)" :!class /Script/Engine.MaterialInstanceDynamic))

(event Custom|Attack
  (bind _returnvalue (Utilities|Time|GetTimeSeconds))
  (if (> _returnvalue (+ (Variables|Default|GetLast%20Attack) (Variables|Default|GetAttack%20Cooldown)))
    (Variables|Default|SetLast%20Attack _returnvalue)
    (Game|SpawnActorfromClass "/Game/Enemies/Projectiles/BP_TurretProjectile.BP_TurretProjectile_C" (Transformation|GetWorldTransform (Variables|Default|GetProjectileSpawn)) "Undefined" 0 0)))

(event Game|Damage|EventAnyDamage
  (params (Damage :type Float%20%28single-precision%29) (DamageType :type Damage%20Type%20Object%20Reference) (InstigatedBy :type Controller%20Object%20Reference) (DamageCauser :type Actor%20Object%20Reference))
  (if (== DamageCauser (Game|GetPlayerCharacter 0))
    (CallFunction|TakeDamage Damage)))

(event EventTick
  (params (DeltaSeconds :type Float%20%28single-precision%29))
  (bind _returnvalue (Transformation|GetActorRotation))
  (if (Variables|Default|GetSearching)
    (Transformation|SetActorRotation (Math|Rotator|MakeRotator (.roll _returnvalue) (.pitch _returnvalue) (+ (.yaw _returnvalue) (* (Math|Random|RandomFloat) 2e+01))))
    (elif (Variables|Default|GetSpotted%20Player)
      (if (< (Variables|Default|GetRange) (Math|Vector|Distance(Vector) (Transformation|GetActorLocation) (Transformation|GetActorLocation (Game|GetPlayerCharacter 0))))
        (CallFunction|FacePlayer)
        (else
          (CallFunction|AimatPlayer)
          (CallFunction|Attack))))))

(fn ConstructionScript)