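; Rooster boss enemy that wanders the navmesh, pursues the player on sight and attacks with bursts of pecks.
; Pawn sensing and Tick-driven flags pick between wandering, chasing with a cooldown-limited long-range charge, and attacking in range, without a behavior tree.
; A dynamic material parameter flashes to telegraph attacks and mark each peck.
; Damage reduces health, and the game mode's alive count tracks its spawn and death.
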(event OnSeePawn(PawnSensing)
  (params (Pawn :type Pawn%20Object%20Reference))
  (Variables|Default|SetSpottedPlayer true)
  (Variables|Default|SetWandering false)
  (Utilities|FlowControl|RetriggerableDelay 0.6)
  (Variables|Default|SetSpottedPlayer false)
  (Variables|Default|SetWandering true))

(event Custom|Chase
  (if (and (> (Utilities|Time|GetTimeSeconds) (+ (Variables|Default|GetLastCharge) (Variables|Default|GetChargeCooldown))) (> (Transformation|GetDistanceTo (Game|GetPlayerCharacter 0)) (Variables|Default|GetChargeOutsideRange)))
    (Variables|/Script/Engine.CharacterMovementComponent|SetMaxWalkSpeed (Variables|Character|GetCharacterMovement) (Variables|Default|GetChargeSpeed))
    (AI|AIMoveTo self (Transformation|GetActorLocation (Game|GetPlayerCharacter 0)) 0 1e+02 true
      (:OnSuccess
        (Variables|Default|SetLastCharge (Utilities|Time|GetTimeSeconds))))
    (elif (> (Utilities|Time|GetTimeSeconds) (+ (Variables|Default|GetLastCharge) (Variables|Default|GetChargeCooldown)))
      (Variables|/Script/Engine.CharacterMovementComponent|SetMaxWalkSpeed (Variables|Character|GetCharacterMovement) (Variables|Default|GetWanderSpeed))
      (AI|AIMoveTo self "0, 0, 0" (Game|GetPlayerCharacter 0) 5.0 true))))

(event Custom|TakeDamage
  (params (Damage :type Float%20%28double-precision%29))
  (bind _output_get (Variables|Default|SetHealth (- (Variables|Default|GetHealth) Damage)))
  (if (<= _output_get 0.0)
    (bind _asbp_third_person_game_mode (Utilities|Casting|CastToBP_ThirdPersonGameMode (Game|GetGameMode)))
    (Variables|/Game/ThirdPerson/Blueprints/BP_ThirdPersonGameMode.BP_ThirdPersonGameMode_C|SetAmount%20Alive _asbp_third_person_game_mode (- (Variables|/Game/ThirdPerson/Blueprints/BP_ThirdPersonGameMode.BP_ThirdPersonGameMode_C|GetAmount%20Alive _asbp_third_person_game_mode) 1))
    (Actor|DestroyActor)))

(event Custom|Attack
  (bind _returnvalue (Utilities|Time|GetTimeSeconds))
  (if (> (Utilities|Time|GetTimeSeconds) (+ (Variables|Default|GetLastPeck) (Variables|Default|GetPeckCooldown)))
    (if (< (Variables|Default|GetPecksThisAttack) (Variables|Default|GetPecksPerAttack))
      (Math|Integer|IncrementInt (Variables|Default|GetPecksThisAttack)
        (:%20%20
          (CallFunction|FlashColour "(R=1.000000,G=0.063658,B=0.567342,A=1.000000)")
          (CallFunction|DoDamage (Game|GetPlayerCharacter 0))
          (Variables|Default|SetLastPeck _returnvalue)))
      (else
        (Variables|Default|SetPecksThisAttack 0)
        (Variables|Default|SetLastAttack _returnvalue)))))

(event Custom|DoDamage
  (params (Target :type Pawn%20Object%20Reference))
  (Game|Damage|ApplyDamage Target (Variables|Default|GetDamage) 0 self))

(event Custom|FlashColour
  (params (Colour :type Linear%20Color%20Structure))
  (bind _returnvalue (Rendering|Material|CreateDynamicMaterialInstance (Variables|Character|GetMesh) 0 0 "None" :!class /Script/Engine.PrimitiveComponent))
  (Rendering|Material|SetVectorParameterValue _returnvalue "RoosterFlashColour" Colour :!class /Script/Engine.MaterialInstanceDynamic)
  (Utilities|FlowControl|RetriggerableDelay 0.1)
  (Rendering|Material|SetVectorParameterValue _returnvalue "RoosterFlashColour" "(R=0.000000,G=0.000000,B=0.000000,A=1.000000)" :!class /Script/Engine.MaterialInstanceDynamic))

(event EventBeginPlay
  (bind _asbp_third_person_game_mode (Utilities|Casting|CastToBP_ThirdPersonGameMode (Game|GetGameMode)))
  (Variables|/Game/ThirdPerson/Blueprints/BP_ThirdPersonGameMode.BP_ThirdPersonGameMode_C|SetAmount%20Alive _asbp_third_person_game_mode (+ (Variables|/Game/ThirdPerson/Blueprints/BP_ThirdPersonGameMode.BP_ThirdPersonGameMode_C|GetAmount%20Alive _asbp_third_person_game_mode) 1))
  (Variables|/Script/Engine.CharacterMovementComponent|SetMaxWalkSpeed (Variables|Character|GetCharacterMovement) (Variables|Default|GetWanderSpeed)))

(event Game|Damage|EventAnyDamage
  (params (Damage :type Float%20%28single-precision%29) (DamageType :type Damage%20Type%20Object%20Reference) (InstigatedBy :type Controller%20Object%20Reference) (DamageCauser :type Actor%20Object%20Reference))
  (CallFunction|TakeDamage Damage))

(event EventTick
  (params (DeltaSeconds :type Float%20%28single-precision%29))
  (Utilities|FlowControl|Sequence
    (:then_0
      (if (Variables|Default|GetSpottedPlayer)
        (if (< (Transformation|GetDistanceTo (Game|GetPlayerCharacter 0)) (Variables|Default|GetAttackRange))
          (if (> (Utilities|Time|GetTimeSeconds) (+ (Variables|Default|GetlastAttack) (Variables|Default|GetattackCooldown)))
            (CallFunction|FlashColour "(R=0.937500,G=0.000000,B=0.000000,A=0.109000)")
            (Utilities|FlowControl|Delay 0.05)
            (Variables|Default|SetAttacking true)
            (else
              (Utilities|FlowControl|Delay 0.2)
              (Variables|Default|SetAttacking false)))
          (else
            (Variables|Default|SetAttacking false)
            (CallFunction|Chase)))
        (elif (Variables|Default|GetWandering)
          _)))
    (:then_1
      (if (Variables|Default|GetAttacking)
        (CallFunction|Attack)
        (elif (and (Variables|Default|GetWandering) (> (Utilities|Time|GetTimeSeconds) (+ (Variables|Default|GetLastWander) (Variables|Default|GetWanderCooldown))))
          (Variables|Default|SetLastWander (Utilities|Time|GetTimeSeconds))
          (bind _randomlocation (Class|NavigationSystemV1|GetRandomLocationinNavigableRadius (Transformation|GetActorLocation) 1e+03 0 0))
          (AI|AIMoveTo self _randomlocation 0 2e+02 true))))))

(fn ConstructionScript)