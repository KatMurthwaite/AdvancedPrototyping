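; AI controller for the ranged chicken enemy that runs its behavior tree and feeds it perception of the player.
; Sight sets target, focus, visibility and last known location, with a short timer on losing sight that presumably clears target and focus.
; Hearing records a target location from any source, while player damage flags TakingDamage and focuses the player.
; Tick uses a delay to reset the damage flag and clear focus.
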(event OnTargetPerceptionUpdated(AIPerception)
  (params (Actor :type Actor%20Object%20Reference) (Stimulus :type AI%20Stimulus%20Structure))
  (CallFunction|SightSense Actor Stimulus)
  (CallFunction|HearingSense 0 Stimulus)
  (CallFunction|DamageSense Actor Stimulus))

(event EventBeginPlay
  (AI|RunBehaviorTree "/Game/CHIEMERIE/Chicken/BehaviourTree/BT_RangedChicken.BT_RangedChicken")
  (bind _astp_third_person_character (Utilities|Casting|CastToTP_ThirdPersonCharacter (Game|GetPlayerCharacter 0)))
  (Variables|Default|SetAs%20TP%20Third%20Person%20Character _astp_third_person_character))

(event EventTick
  (params (DeltaSeconds :type Float%20%28single-precision%29))
  (if (Variables|Default|GetTakingDamage)
    (Utilities|FlowControl|Delay 3.0)
    (bind _output_get (Variables|Default|SetTakingDamage false))
    (AI|Components|Blackboard|SetValueasBool (Variables|Default|GetBlackboard) (Utilities|Name|MakeLiteralName "TakingDamage") _output_get)
    (AI|ClearFocus)))

(fn ConstructionScript)

(fn SightSense
  (params (Actor :type Actor%20Object%20Reference) (Stimulus :type AI%20Stimulus%20Structure))
  (bind (_age _expirationage _strength _stimuluslocation _receiverlocation _tag _bsuccessfullysensed) (Utilities|Struct|BreakAIStimulus Stimulus))
  (bind _returnvalue (Class|AIPerceptionSystem|GetSenseClassforStimulus Stimulus))
  (if (and (== Actor (Game|GetPlayerCharacter 0)) (== _returnvalue "/Script/AIModule.AISense_Sight"))
    (if _bsuccessfullysensed
      (AI|Components|Blackboard|SetValueasObject (Variables|Default|GetBlackboard) (Utilities|Name|MakeLiteralName "TargetActor") (Variables|Default|GetAs%20TP%20Third%20Person%20Character))
      (AI|SetFocus (Variables|Default|GetAs%20TP%20Third%20Person%20Character))
      (Utilities|Time|ClearandInvalidateTimerbyHandle (Variables|Default|GetLoose%20Target%20Timer))
      (Variables|Default|SetCanSeeEnemy true)
      (AI|Components|Blackboard|SetValueasBool (Variables|Default|GetBlackboard) (Utilities|Name|MakeLiteralName "CanSeeEnemy") true)
      (AI|Components|Blackboard|SetValueasVector (Variables|Default|GetBlackboard) (Utilities|Name|MakeLiteralName "LastKnownLocation") _stimuluslocation)
      (else
        (Variables|Default|SetCanSeeEnemy false)
        (bind _returnvalue_2 (Utilities|Time|SetTimerbyEvent (EventDispatchers|CreateEvent :!event RangedControllerBPAutoGenFunc) 0.5))
        (Variables|Default|SetLoose%20Target%20Timer _returnvalue_2)
        (AI|Components|Blackboard|SetValueasVector (Variables|Default|GetBlackboard) (Utilities|Name|MakeLiteralName "LastKnownLocation") _stimuluslocation)
        (AI|Components|Blackboard|SetValueasBool (Variables|Default|GetBlackboard) (Utilities|Name|MakeLiteralName "CanSeeEnemy") false)))))

(fn RangedControllerBPAutoGenFunc
  (AI|Components|Blackboard|SetValueasObject (Variables|Default|GetBlackboard) (Utilities|Name|MakeLiteralName "TargetActor") 0)
  (AI|ClearFocus))

(fn HearingSense
  (params (Actor :type Actor%20Object%20Reference) (Stimulus :type AI%20Stimulus%20Structure))
  (bind _returnvalue (Class|AIPerceptionSystem|GetSenseClassforStimulus Stimulus))
  (if (== _returnvalue "/Script/AIModule.AISense_Hearing")
    (AI|Components|Blackboard|SetValueasVector (Variables|Default|GetBlackboard) (Utilities|Name|MakeLiteralName "TargetLocation") (.StimulusLocation (Utilities|Struct|BreakAIStimulus Stimulus)))))

(fn DamageSense
  (params (Actor :type Actor%20Object%20Reference) (Stimulus :type AI%20Stimulus%20Structure))
  (bind _returnvalue (Class|AIPerceptionSystem|GetSenseClassforStimulus Stimulus))
  (if (and (== Actor (Game|GetPlayerCharacter 0)) (== _returnvalue "/Script/AIModule.AISense_Damage"))
    (bind _output_get (Variables|Default|SetTakingDamage true))
    (AI|Components|Blackboard|SetValueasBool (Variables|Default|GetBlackboard) (Utilities|Name|MakeLiteralName "TakingDamage") _output_get)
    (AI|SetFocus (Variables|Default|GetAs%20TP%20Third%20Person%20Character))))